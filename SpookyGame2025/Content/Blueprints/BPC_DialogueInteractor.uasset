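; BPC_DialogueInteractor is an actor component that detects dialogue-interactable objects in front of its owner.
; On Interact, it gets the owner's position and look direction through interface messages and runs a debug-drawn sphere trace out to Range.
; If the hit actor has a BPC_DialogueInteractable component, it only prints a debug string; no dialogue is started here.
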(event Custom|Interact
  (bind _returnvalue (Components|GetOwner))
  (bind _lookdirection (Class|BPICharacter|GetLookDirection(Message) _returnvalue))
  (bind _position (Class|BPICharacter|GetPosition(Message) _returnvalue))
  (bind (_outhit _returnvalue_2) (Collision|SphereTraceForObjects _position (+ (* (Variables|Default|GetRange) _lookdirection) _position) 1e+01 (Utilities|Array|MakeArray "ObjectTypeQuery1" "ObjectTypeQuery2" "ObjectTypeQuery4") false 0 "ForDuration"))
  (if _returnvalue_2
    (if (Utilities|IsValid (Actor|GetComponentbyClass (.HitActor (Collision|BreakHitResult _outhit)) "/Game/Blueprints/BPC_DialogueInteractable.BPC_DialogueInteractable_C"))
      (Development|PrintString "Found Interactable Object"))))

(event EventBeginPlay)

(event EventTick
  (params (DeltaSeconds :type Float%20%28single-precision%29)))