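; BPC_DialogueInteractor is a component that lets its owner interact with objects or start dialogue with them.
; On Interact, it sphere-traces up to Range along the owner's look direction, using position and direction from message calls, with debug drawing.
; Hit actors implementing Interactable receive an interact message.
; Otherwise, a BP_DialogueInteractableBox hit is passed to the first-person character's dialogue manager to enter dialogue.
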(event Custom|Interact
  (bind _returnvalue (Components|GetOwner))
  (bind _lookdirection (Class|BPICharacter|GetLookDirection(Message) _returnvalue))
  (bind _position (Class|BPICharacter|GetPosition(Message) _returnvalue))
  (bind (_outhit _returnvalue_2) (Collision|SphereTraceForObjects _position (+ (* (Variables|Default|GetRange) _lookdirection) _position) 1e+01 (Utilities|Array|MakeArray "ObjectTypeQuery1" "ObjectTypeQuery2" "ObjectTypeQuery4" "ObjectTypeQuery3") false 0 "ForDuration"))
  (if _returnvalue_2
    ;[0.15 0.15 0.15 0.5] Interactors
    (if (Utilities|DoesObjectImplementInterface (.HitActor (Collision|BreakHitResult _outhit)) "/Script/SpookyGame2025.Interactable")
      (Class|Interactable|InteractwithObject(Message) (.HitActor (Collision|BreakHitResult _outhit)) (Components|GetOwner))
      (else
        (bind _asbp_dialogue_interactable_box (Utilities|Casting|CastToBP_DialogueInteractableBox (.HitActor (Collision|BreakHitResult _outhit))))
        (Development|PrintString "Found Dialogue Interactable")
        (bind _asbp_first_person_character (Utilities|Casting|CastToBP_FirstPersonCharacter (Components|GetOwner)))
        (Default|EnterDialogue (Variables|/Game/FirstPerson/Blueprints/BP_FirstPersonCharacter.BP_FirstPersonCharacter_C|GetBPC_DialogueManager _asbp_first_person_character) _asbp_dialogue_interactable_box)))))

(event EventBeginPlay)

(event EventTick
  (params (DeltaSeconds :type Float%20%28single-precision%29)))