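; Dialogue manager component that runs branching conversations with dialogue interactables.
; Entering or ending dialogue toggles the dialogue widget and swaps input mapping through the game manager's controller.
; Progressing steps through the current block's lines and ends the conversation on a last line without choices; otherwise the chosen end choice jumps to another block by index.
; Getter functions expose the current line, end-of-block state and choice text with a validity flag.
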(event Custom|EnterDialogue
  (params (DialogueInteractable :type BP%20Dialogue%20Interactable%20Box%20Object%20Reference))
  (Variables|Default|SetIsInDialogue true)
  (bind _output_get (Variables|Default|SetCurrentDialogueInteractable DialogueInteractable))
  (Variables|Default|SetCurrentDialogueIndex 0)
  (Variables|Default|SetCurrentDialogueBlock (Utilities|Array|Get(acopy) (Variables|/Game/Blueprints/Dialogue/BP_DialogueInteractableBox.BP_DialogueInteractableBox_C|GetDialogueBlocks _output_get) (Variables|Default|GetCurrentDialogueIndex)))
  (bind _returnvalue (Actor|GetActorOfClass "/Game/Blueprints/BP_GameManager.BP_GameManager_C"))
  (Default|SetInputMapping (Variables|/Game/Blueprints/BP_GameManager.BP_GameManager_C|GetController _returnvalue) "/Game/Input/IMC_InDialogue.IMC_InDialogue")
  (UserInterface|Viewport|AddtoViewport (Variables|Default|GetDialogueWidget) 0))

(event Custom|EndDialogue
  (Variables|Default|SetCurrentDialogueInteractable 0)
  (Variables|Default|SetCurrentDialogueBlock "")
  (Variables|Default|SetIsInDialogue false)
  (bind _returnvalue (Actor|GetActorOfClass "/Game/Blueprints/BP_GameManager.BP_GameManager_C"))
  (Default|SetInputMapping (Variables|/Game/Blueprints/BP_GameManager.BP_GameManager_C|GetController _returnvalue) "/Game/Input/IMC_Default.IMC_Default")
  (Widget|RemovefromParent (Variables|Default|GetDialogueWidget)))

(event Custom|ProgressDialogue
  (bind _isatend (CallFunction|GetIsatEnd))
  (if _isatend
    (bind _haschoices (CallFunction|HasChoices))
    (if (not _haschoices)
      (CallFunction|EndDialogue))
    (else
      (Variables|Default|SetCurrentDialogueIndex (+ (Variables|Default|GetCurrentDialogueIndex) 1)))))

(event Custom|ChooseChoice
  (params (ChoiceIndex :type Integer))
  (bind _isatend (CallFunction|GetIsatEnd))
  (if _isatend
    (Variables|Default|SetCurrentDialogueBlock (Utilities|Array|Get(acopy) (Variables|/Game/Blueprints/Dialogue/BP_DialogueInteractableBox.BP_DialogueInteractableBox_C|GetDialogueBlocks (Variables|Default|GetCurrentDialogueInteractable)) (.NextDialogueBlock (Utilities|Struct|BreakBPS_Choice (Utilities|Array|Get(acopy) (.EndChoices (Utilities|Struct|BreakBPS_DialogueBlock (Variables|Default|GetCurrentDialogueBlock))) ChoiceIndex)))))
    (Variables|Default|SetCurrentDialogueIndex 0)
    (else
      (Development|PrintString "Chose Choice while not at end of Dialogue block"))))

(event EventBeginPlay
  (bind _returnvalue (UserInterface|CreateWidget "/Game/UI/W_DialogueUI.W_DialogueUI_C"))
  (Variables|Default|SetDialogueWidget _returnvalue))

(event EventTick
  (params (DeltaSeconds :type Float%20%28single-precision%29)))

(fn GetCurrentDialogue
  (return (Utilities|Array|Get(acopy) (.Dialogue (Utilities|Struct|BreakBPS_DialogueBlock (Variables|Default|GetCurrentDialogueBlock))) (Variables|Default|GetCurrentDialogueIndex))))

(fn GetIsatEnd
  (return (== (Variables|Default|GetCurrentDialogueIndex) (- (Utilities|Array|Length (.Dialogue (Utilities|Struct|BreakBPS_DialogueBlock (Variables|Default|GetCurrentDialogueBlock)))) 1))))

(fn GetChoiceText
  (params (Index :type Integer))
  (bind _currentdialogueblock (Variables|Default|GetCurrentDialogueBlock))
  (bind _endchoices (Utilities|Struct|BreakBPS_DialogueBlock _currentdialogueblock))
  (bind _isatend (CallFunction|GetIsatEnd))
  (if _isatend
    (if (< Index (Utilities|Array|Length _endchoices))
      (return (.ChoiceText (Utilities|Struct|BreakBPS_Choice (Utilities|Array|Get(acopy) _endchoices Index))) true)
      (else
        (return "" false)))
    (else
      (return "" false))))

(fn HasChoices
  (return (> (Utilities|Array|Length (.EndChoices (Utilities|Struct|BreakBPS_DialogueBlock (Variables|Default|GetCurrentDialogueBlock)))) 0)))