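; BPC_DialogueManager is a dialogue manager component that tracks the active conversation with a dialogue interactable.
; EnterDialogue flags dialogue as active, stores the interactable, resets the index and caches the first entry of its DialogueBlocks.
; EndDialogue clears the interactable, current block and active flag.
; ProgressDialogue is an empty stub, with a note planning input-method switching and basic UI.
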(event Custom|EnterDialogue
  (params (DialogueInteractable :type BP%20Dialogue%20Interactable%20Box%20Object%20Reference))
  (Variables|Default|SetIsInDialogue true)
  (bind _output_get (Variables|Default|SetCurrentDialogueInteractable DialogueInteractable))
  (Variables|Default|SetCurrentDialogueIndex 0)
  (Variables|Default|SetCurrentDialogueBlock (Utilities|Array|Get(acopy) (Variables|/Game/Blueprints/BP_DialogueInteractableBox.BP_DialogueInteractableBox_C|GetDialogueBlocks _output_get) (Variables|Default|GetCurrentDialogueIndex))))

(event Custom|EndDialogue
  (Variables|Default|SetCurrentDialogueInteractable 0)
  (Variables|Default|SetCurrentDialogueBlock "")
  (Variables|Default|SetIsInDialogue false))

(event Custom|ProgressDialogue
  ;[0.15 0.15 0.15 0.5] add function for changing input method and add basic UI
)

(event EventBeginPlay)

(event EventTick
  (params (DeltaSeconds :type Float%20%28single-precision%29)))